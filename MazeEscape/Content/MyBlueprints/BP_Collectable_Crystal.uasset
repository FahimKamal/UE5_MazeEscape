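; BP_Collectable_Crystal is an interactable crystal pickup that triggers the win screen when the player collects it.
; LookAtObject always reports it as interactable and returns a press-E prompt.
; InteractwithObject adds its ItemInfo to the player's inventory, shows an important HUD message, adds WBP_WinScreen to the viewport, then destroys the actor.
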(event `/Game/MyBlueprints/BPI_Interaction.InteractWithObject`
  (params (`Player Character` :type "/Game/FirstPerson/Blueprints/BP_FirstPersonCharacter_default Object Reference"))
  (`/Game/FirstPerson/Blueprints/BP_FirstPersonCharacter_default.AddInventory` `Player Character` (`self.Item Info`) 1)
  (`/Game/FirstPerson/Blueprints/BP_MainHUD.Show Interaction Message` (`/Game/FirstPerson/Blueprints/BP_FirstPersonCharacter_default.MainHUD` `Player Character`) "The crystal added in your inventory." true)
  (bind _returnvalue (`|CreateWidget` "/Game/UI/WBP_WinScreen.WBP_WinScreen_C"))
  (`UserWidget.AddToViewport` _returnvalue 0)
  (`self.K2_DestroyActor`))

(fn `LookAtObject`
  (params (`First Person Character` :type "/Game/FirstPerson/Blueprints/BP_FirstPersonCharacter_default Object Reference"))
  (returns (`CanBeInteracted?` :type Boolean) (Message :type Text))
  (return true "Press 'E' to collect the The mysteries crystal."))

(fn `UserConstructionScript`
  (`parent.UserConstructionScript`))