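; BP_Monitor is an interactable computer monitor that can be locked behind a password item or hold an item to collect.
; Interacting while locked consumes the matching inventory item and fires CallOnComputerUnlocked; while unlocked, it hands over any stored item, with HUD feedback.
; Light controller events drive PowerStateChange, also run at construction after creating the screen's dynamic material.
; Power affects the look-at prompt, but interaction itself does not check it.
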(event `self.LightController.OnLightStateChanged`
  (params (`Light On` :type Boolean))
  (bind _output_get (set `self.IsPowerOn?` `Light On`))
  (`self.PowerStateChange` _output_get))

(event `/Game/MyBlueprints/BPI_Interaction.InteractWithObject`
  (params (`Player Character` :type "/Game/FirstPerson/Blueprints/BP_FirstPersonCharacter_default Object Reference"))
  (bind _mainhud (`/Game/FirstPerson/Blueprints/BP_FirstPersonCharacter_default.MainHUD` `Player Character`))
  ; When the computer is locked and player has a key to unlock the computer.
  (if (`self.IsInteractable?`)
    (if (`self.IsLocked?`)
      (bind _da_item (`self.DA Item`)
        (:`then`
          (bind _ispresent_ (`/Game/FirstPerson/Blueprints/BP_FirstPersonCharacter_default.CheckInventory` `Player Character` _da_item))
          (if _ispresent_
            (`/Game/FirstPerson/Blueprints/BP_MainHUD.Show Interaction Message` _mainhud "Computer is unlocked and door is unlocked." true)
            (`/Game/FirstPerson/Blueprints/BP_FirstPersonCharacter_default.RemoveInventory` `Player Character` (`self.DA Item`) 1)
            (set `self.IsLocked?` false)
            (`self.OnComputerUnlocked`)
            (else
              (`/Game/FirstPerson/Blueprints/BP_MainHUD.Show Interaction Message` _mainhud "Find password to unlock the computer." true))))
        (:`else`))
      (else
        ; When the computer is not locked and there is a key in here.
        (bind _da_item_2 (`self.DA Item`)
          (:`then`
            (`/Game/FirstPerson/Blueprints/BP_FirstPersonCharacter_default.AddInventory` `Player Character` _da_item_2 1)
            (set `self.DA Item` null)
            (`/Game/FirstPerson/Blueprints/BP_MainHUD.Show Interaction Message` _mainhud "You have collected a password." true))
          (:`else`
            (`/Game/FirstPerson/Blueprints/BP_MainHUD.Show Interaction Message` (`/Game/FirstPerson/Blueprints/BP_FirstPersonCharacter_default.MainHUD` `Player Character`) "Nothing found on the computer." true)))))))

(fn `LookAtObject`
  (params (`First Person Character` :type "/Game/FirstPerson/Blueprints/BP_FirstPersonCharacter_default Object Reference"))
  (returns (`CanBeInteracted?` :type Boolean) (Message :type Text))
  (if (`self.IsInteractable?`)
    (if (`self.IsPowerOn?`)
      (if (`self.IsLocked?`)
        (return true "Computer is locked.")
        (else
          (return true "Press 'E' to interact with the computer.")))
      (else
        (return true "Computer needs power to work.")))))

(fn `UserConstructionScript`
  (bind _returnvalue (`PrimitiveComponent.CreateDynamicMaterialInstance` (`self.Screen`) 0 null "None"))
  (set `self.Material` _returnvalue)
  (`self.PowerStateChange` (`self.IsPowerOn?`)))