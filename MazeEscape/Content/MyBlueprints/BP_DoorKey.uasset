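; BP_DoorKey is a key pickup that the player collects by interacting with it.
; LookAtObject always reports it as interactable and returns a prompt message about collecting the key.
; InteractwithObject adds one of its ItemInfo to the player character's inventory, then destroys the actor.
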(event `/Game/MyBlueprints/BPI_Interaction.InteractWithObject`
  (params (`Player Character` :type "/Game/FirstPerson/Blueprints/BP_FirstPersonCharacter_default Object Reference"))
  (`/Game/FirstPerson/Blueprints/BP_FirstPersonCharacter_default.AddInventory` `Player Character` (`self.Item Info`) 1)
  (`self.K2_DestroyActor`))

(fn `LookAtObject`
  (params (`First Person Character` :type "/Game/FirstPerson/Blueprints/BP_FirstPersonCharacter_default Object Reference"))
  (returns (`CanBeInteracted?` :type Boolean) (Message :type Text))
  (return true "To collected the key."))

(fn `UserConstructionScript`
  (`parent.UserConstructionScript`))