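; An interactable lift that carries its floor between a lower and an upper point.
; Interaction signals lift start, then after a short delay plays or reverses a timeline that scales the upper point's relative Z by playback position to move the floor.
; When the timeline finishes, it signals lift stop and updates the upper-point flag from its direction, which also selects the up or down look-at prompt.
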(event `LiftMovement`
  (if (`self.OnUpperpoint?`)
    (bind (_direction _position) (`Timeline|Timeline-liftmovement` :!via `Reverse` :!label _label)
      (:`Update`
        (bind (_returnvalue_x _returnvalue_y _returnvalue_z) (`KismetMathLibrary.BreakVector` (* (`SceneComponent.RelativeLocation` (`self.LiftUpperPoint`)) _position)))
        (`SceneComponent.K2_SetRelativeLocation` (`self.LiftFloor`) (`KismetMathLibrary.MakeVector` 0.0 0.0 _returnvalue_z) false false))
      (:`Finished`
        (`self.OnLiftStop`)
        (switch `ETimelineDirection` _direction
          (:`Forward`
            (set `self.OnUpperpoint?` true))
          (:`Backward`
            (set `self.OnUpperpoint?` false)))))
    (else
      (goto _label))))

(event `/Game/MyBlueprints/BPI_Interaction.InteractWithObject`
  (params (`Player Character` :type "/Game/FirstPerson/Blueprints/BP_FirstPersonCharacter_default Object Reference"))
  (`self.OnLiftStart`)
  (`KismetSystemLibrary.Delay` 1.2)
  (`self.LiftMovement`))

(fn `LookAtObject`
  (params (`First Person Character` :type "/Game/FirstPerson/Blueprints/BP_FirstPersonCharacter_default Object Reference"))
  (returns (`CanBeInteracted?` :type Boolean) (Message :type Text))
  (if (`self.OnUpperpoint?`)
    (return true "Press 'E' to go down.")
    (else
      (return true "Press 'E' to go up."))))

(fn `UserConstructionScript`)