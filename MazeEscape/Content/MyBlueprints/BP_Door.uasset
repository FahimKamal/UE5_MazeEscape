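; BP_Door is a sliding door actor that opens automatically when the player character overlaps it and closes when they leave.
; OpenDoor plays a timeline that moves the Door component's relative location along X, scaled by the timeline's Position track.
; CloseDoor reverses the same timeline, so the door slides back from wherever it currently is.
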(event `Open Door`
  (bind (_direction _position) (`Timeline|DoorOpenTimeline` :!label _label)
    (:`Update`
      (`SceneComponent.K2_SetRelativeLocation` (`self.Door`) (* (160.0 0.0 0.0) _position) false false))))

(event `Close Door`
  (goto _label :!via `Reverse`))

(event `self.ReceiveActorBeginOverlap`
  (params (OtherActor :type "Actor Object Reference"))
  (if (== OtherActor (`GameplayStatics.GetPlayerCharacter` 0))
    (`self.Open Door`)))

(event `self.ReceiveActorEndOverlap`
  (params (OtherActor :type "Actor Object Reference"))
  (if (== OtherActor (`GameplayStatics.GetPlayerCharacter` 0))
    (`self.Close Door`)))

(fn `UserConstructionScript`)