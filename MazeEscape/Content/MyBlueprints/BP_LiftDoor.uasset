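; Lift door actor that players open by interacting, with a lock released by a key item or a power generator.
; A timeline slides two panels apart, then reverses after a short delay; lift start and stop events also close and open it.
; Unlocking by key consumes the item and shows a HUD message.
; A dynamic material colors the lock indicator, and LookAtObject supplies prompts matching the lock state.
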(event `self.ReceiveBeginPlay`
  (bind _asbp_first_person_character_default (cast `/Game/FirstPerson/Blueprints/BP_FirstPersonCharacter_default` (`GameplayStatics.GetPlayerCharacter` 0)))
  (set `self.As BP First Person Character Default` _asbp_first_person_character_default))

(event `Open Door`
  ;[0.8281 0.7088 0.1078 0.5] Door open and close logic
  (bind (_direction _position) (`Timeline|DoorOpenTimeline` :!label _label)
    (:`Update`
      (`SceneComponent.K2_SetRelativeLocation` (`self.Door-L`) (`KismetMathLibrary.VLerp` (0.0 0.0 0.0) (-130.0 0.0 0.0) _position) false false)
      (`SceneComponent.K2_SetRelativeLocation` (`self.Door-R`) (`KismetMathLibrary.VLerp` (260.0 10.0 0.0) (395.0 10.0 0.0) _position) false false))
    (:`Finished`
      (switch `ETimelineDirection` _direction
        (:`Forward`
          (`KismetSystemLibrary.Delay` 3.0)
          (`self.Close Door`))))))

(event `Close Door`
  ;[0.8281 0.7088 0.1078 0.5] Door open and close logic
  (goto _label :!via `Reverse`))

(event `self.ReceiveActorBeginOverlap`
  (params (OtherActor :type "Actor Object Reference")))

(event `Unlock Door`
  ;[0.3559 0.6458 0 0.5] Door lock and unlock logic
  (set `self.IsDoorLocked?` false)
  (`MaterialInstanceDynamic.SetVectorParameterValue` (`self.Lock Indicator Mat`) "Basic Color" (struct :`R` 0.181106 :`G` 1.0 :`A` 1.0)))

(event `self.ReceiveActorEndOverlap`
  (params (OtherActor :type "Actor Object Reference")))

(event `Lock Door`
  ;[0.3559 0.6458 0 0.5] Door lock and unlock logic
  (set `self.IsDoorLocked?` true)
  (`MaterialInstanceDynamic.SetVectorParameterValue` (`self.Lock Indicator Mat`) "Basic Color" (struct :`R` 1.0 :`G` 0.09287 :`A` 1.0)))

(event `self.InteractWithObject`
  (params (`Player Character` :type "/Game/FirstPerson/Blueprints/BP_FirstPersonCharacter_default Object Reference"))
  ;[0.8281 0.7088 0.1078 0.5] When player try to interact with this object.
  (if (`self.IsDoorLocked?`)
    (`self.Key Item`
      (:`then`
        (bind _ispresent_ (`/Game/FirstPerson/Blueprints/BP_FirstPersonCharacter_default.CheckInventory` `Player Character` (`self.Key Item`)))
        (if _ispresent_
          (`self.Unlock Door`)
          (`/Game/FirstPerson/Blueprints/BP_FirstPersonCharacter_default.RemoveInventory` `Player Character` (`self.Key Item`) 1)
          (`/Game/FirstPerson/Blueprints/BP_MainHUD.Show Interaction Message` (`/Game/FirstPerson/Blueprints/BP_FirstPersonCharacter_default.MainHUD` `Player Character`) "Door unlocked." false)))
      (:`else`))
    (else
      (`self.Open Door`))))

(event `self.PowerGenerator.OnGeneratorTurnOn`
  (params (TurnedOn :type Boolean))
  (`self.Unlock Door`))

(event `self.BP_Lift.OnLiftStart`
  (`self.Close Door`))

(event `self.BP_Lift.OnLiftStop`
  (`self.Open Door`))

(fn `LookAtObject`
  (params (`First Person Character` :type "/Game/FirstPerson/Blueprints/BP_FirstPersonCharacter_default Object Reference"))
  (returns (`CanBeInteracted?` :type Boolean) (Message :type Text))
  (if (`self.IsDoorLocked?`)
    (bind _key_item (`self.Key Item`)
      (:`then`
        (bind _ispresent_ (`/Game/FirstPerson/Blueprints/BP_FirstPersonCharacter_default.CheckInventory` `First Person Character` _key_item))
        (if _ispresent_
          (return true "Press 'E' to use the key to unlock the lift.")
          (else
            (return true "You need a key to open the lift."))))
      (:`else`
        (return true "Lift need power. Turn on the generator.")))
    (else
      (return true "Press 'E' to open the lift."))))

(fn `UserConstructionScript`
  (bind _lock_indicator_mat (`self.Lock Indicator Mat`))
  (bind _returnvalue (`PrimitiveComponent.CreateDynamicMaterialInstance` (`self.Look Indicator`) 0 null "None"))
  (set `self.Lock Indicator Mat` _returnvalue)
  (if (`self.IsDoorLocked?`)
    (`MaterialInstanceDynamic.SetVectorParameterValue` _lock_indicator_mat "Basic Color" (struct :`R` 1.0 :`G` 0.09287 :`A` 1.0))
    (else
      (`MaterialInstanceDynamic.SetVectorParameterValue` _lock_indicator_mat "Basic Color" (struct :`R` 0.181106 :`G` 1.0 :`A` 1.0)))))