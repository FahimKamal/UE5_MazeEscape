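; BP_PowerGenerator is a power generator actor whose cell cases and pipes show its on or off state.
; The Construction Script creates dynamic materials and sets them from GeneratorState: case colors and brightness, plus pipe brightness and scroll speed.
; One cell case material instance is shared across all three cases, while Pipe1 and Pipe7 get their own.
; PositionPowerCell spawns a BP_PowerCell at a target's transform but is not called here.
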(fn `PipePowerOff`
  (params (TargetMaterial :type "MaterialInstanceDynamic Object Reference"))
  (`MaterialInstanceDynamic.SetScalarParameterValue` TargetMaterial "SpeedY_A" 0.0)
  (`MaterialInstanceDynamic.SetScalarParameterValue` TargetMaterial "SpeedY_B" 0.0)
  (`MaterialInstanceDynamic.SetScalarParameterValue` TargetMaterial "Brightness" 0.0))

(fn `PipePowerOn`
  (params (`Target Material` :type "MaterialInstanceDynamic Object Reference"))
  (`MaterialInstanceDynamic.SetScalarParameterValue` `Target Material` "SpeedY_A" 0.22)
  (`MaterialInstanceDynamic.SetScalarParameterValue` `Target Material` "SpeedY_B" 0.25)
  (`MaterialInstanceDynamic.SetScalarParameterValue` `Target Material` "Brightness" 3.0))

(fn `PositionPowerCell`
  (params (Target :type "SceneComponent Object Reference"))
  (`|SpawnActorFromClass` "/Game/MyBlueprints/PowerGenerator/BP_PowerCell.BP_PowerCell_C" (`SceneComponent.K2_GetComponentToWorld` Target) "Undefined" "MultiplyWithRoot" self null))

(fn `PowerStateOfCellCase`
  (params (`IsPowerOn?` :type Boolean))
  (bind _cellcasematerial (`self.CellCaseMaterial`))
  (if `IsPowerOn?`
    (`MaterialInstanceDynamic.SetVectorParameterValue` _cellcasematerial "PrimaryColor" (struct :`R` 0.180392 :`G` 0.913726 :`B` 0.121569 :`A` 1.0))
    (`MaterialInstanceDynamic.SetVectorParameterValue` _cellcasematerial "SecondaryColor" (struct :`R` 0.023529 :`G` 0.203922 :`B` 0.172549 :`A` 1.0))
    (`MaterialInstanceDynamic.SetScalarParameterValue` _cellcasematerial "Brightness" 3.0)
    (else
      (`MaterialInstanceDynamic.SetVectorParameterValue` _cellcasematerial "PrimaryColor" (struct :`R` 1.0 :`G` 0.043376 :`A` 1.0))
      (`MaterialInstanceDynamic.SetVectorParameterValue` _cellcasematerial "SecondaryColor" (struct :`R` 1.0 :`G` 0.043376 :`A` 1.0))
      (`MaterialInstanceDynamic.SetScalarParameterValue` _cellcasematerial "Brightness" 0.2)))
  (`PrimitiveComponent.SetMaterial` (`self.Cell Case2`) 0 _cellcasematerial)
  (`PrimitiveComponent.SetMaterial` (`self.Cell Case3`) 0 _cellcasematerial))

(fn `PowerStateOfPipes`
  (params (`IsPowerOn?` :type Boolean))
  (bind _small_pipe (`self.Small Pipe`))
  (bind _big_pipe (`self.Big Pipe`))
  (if `IsPowerOn?`
    (`self.PipePowerOn` _big_pipe)
    (`self.PipePowerOn` _small_pipe)
    (else
      (`self.PipePowerOff` _big_pipe)
      (`self.PipePowerOff` _small_pipe))))

(fn `UserConstructionScript`
  (`|ExecutionSequence`
    (:`then_0`
      (bind _returnvalue (`PrimitiveComponent.CreateDynamicMaterialInstance` (`self.Cell Case`) 0 null "None"))
      (set `self.CellCaseMaterial` _returnvalue)
      (switch `/Game/MyBlueprints/PowerGenerator/E_GeneratorState` (`self.GeneratorState`)
        (:`NewEnumerator0`
          (`self.PowerStateOfCellCase` false))
        (:`NewEnumerator1`
          (`self.PowerStateOfCellCase` true))))
    (:`then_1`
      (bind _returnvalue_2 (`PrimitiveComponent.CreateDynamicMaterialInstance` (`self.Pipe1`) 0 null "None"))
      (set `self.Big Pipe` _returnvalue_2)
      (bind _returnvalue_3 (`PrimitiveComponent.CreateDynamicMaterialInstance` (`self.Pipe7`) 0 null "None"))
      (set `self.Small Pipe` _returnvalue_3)
      (switch `/Game/MyBlueprints/PowerGenerator/E_GeneratorState` (`self.GeneratorState`)
        (:`NewEnumerator0`
          (`self.PowerStateOfPipes` false))
        (:`NewEnumerator1`
          (`self.PowerStateOfPipes` true))))))