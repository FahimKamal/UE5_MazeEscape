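; BP_Monitor2 is a monitor Blueprint whose screen power state follows a light controller.
; Construction creates a dynamic material instance on the Screen and applies the initial power state, or hides the screen in game when ScreenActive is false.
; LightController's OnLightStateChanged event copies the light state into IsPowerOn and calls PowerStateChange, whose body is not shown here.
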(event `self.LightController.OnLightStateChanged`
  (params (`Light On` :type Boolean))
  (bind _output_get (set `self.IsPowerOn?` `Light On`))
  (`self.PowerStateChange` _output_get))

(fn `UserConstructionScript`
  (if (`self.ScreenActive?`)
    (bind _returnvalue (`PrimitiveComponent.CreateDynamicMaterialInstance` (`self.Screen`) 0 null "None"))
    (set `self.Material` _returnvalue)
    (`self.PowerStateChange` (`self.IsPowerOn?`))
    (else
      (`SceneComponent.SetHiddenInGame` (`self.Screen`) true false))))