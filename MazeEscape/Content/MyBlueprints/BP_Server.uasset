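; BP_Server is a server prop whose indicator lights react to power state changes.
; The construction script creates red, white and green dynamic material instances, shares each across same-colored light components, then applies the initial power state.
; LightController's OnLightStateChanged event updates IsPowerOn and calls PowerStateChange.
; That function toggles Glow Intensity on white and green materials only, leaving red untouched.
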(event `self.LightController.OnLightStateChanged`
  (params (`Light On` :type Boolean))
  (bind _output_get (set `self.IsPowerOn?` `Light On`))
  (`self.PowerStateChange` _output_get))

(fn `PowerStateChange`
  (params (`IsPowerOn?` :type Boolean))
  (if `IsPowerOn?`
    (`MaterialInstanceDynamic.SetScalarParameterValue` (`self.mat_white`) "Glow Intensity" 1.0)
    (`MaterialInstanceDynamic.SetScalarParameterValue` (`self.mat_green`) "Glow Intensity" 1.0)
    (else
      (`MaterialInstanceDynamic.SetScalarParameterValue` (`self.mat_white`) "Glow Intensity" 0.0)
      (`MaterialInstanceDynamic.SetScalarParameterValue` (`self.mat_green`) "Glow Intensity" 0.0))))

(fn `UserConstructionScript`
  (`|ExecutionSequence`
    (:`then_0`
      (bind _returnvalue (`PrimitiveComponent.CreateDynamicMaterialInstance` (`self.ServerLights6_red`) 0 null "None"))
      (bind _output_get (set `self.Mat_red` _returnvalue))
      (`PrimitiveComponent.SetMaterial` (`self.ServerLights4_red`) 0 _output_get))
    (:`then_1`
      (bind _returnvalue_2 (`PrimitiveComponent.CreateDynamicMaterialInstance` (`self.ServerLights5_white`) 0 null "None"))
      (bind _output_get_2 (set `self.mat_white` _returnvalue_2))
      (`PrimitiveComponent.SetMaterial` (`self.ServerLights3_white`) 0 _output_get_2)
      (`PrimitiveComponent.SetMaterial` (`self.ServerLights_white`) 0 _output_get_2))
    (:`then_2`
      (bind _returnvalue_3 (`PrimitiveComponent.CreateDynamicMaterialInstance` (`self.ServerLights_green`) 0 null "None"))
      (bind _output_get_3 (set `self.mat_green` _returnvalue_3))
      (`PrimitiveComponent.SetMaterial` (`self.ServerLights1_green`) 0 _output_get_3))
    (:`then_3`
      (`self.PowerStateChange` (`self.IsPowerOn?`)))))